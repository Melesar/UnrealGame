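; TextPC is a player controller that lets a client without a pawn request a respawn.
; On the Resp input, only the remote side acts: it prints a debug message if a pawn is controlled, otherwise it calls the respawn request event.
; That event proceeds only with authority, casting the game mode and calling its Respawn function with this controller.
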(event `InputAction|Resp`
  (params (Key :type "Key Structure"))
  (:`Pressed`
    (`/Engine/EditorBlueprintResources/ActorMacros.Switch Has Authority`
      (:`Remote`
        (`/Engine/EditorBlueprintResources/StandardMacros.IsValid` (`self.K2_GetPawn` self)
          (:`Is Valid`
            (`KismetSystemLibrary.PrintString` "Pc client is contolliing"))
          (:`Is Not Valid`
            (`self.requestGMRespawm`)))))))

(event `requestGMRespawm`
  (bind _returnvalue (`GameplayStatics.GetGameMode`))
  (`/Engine/EditorBlueprintResources/ActorMacros.Switch Has Authority`
    (:`Authority`
      (`/Engine/EditorBlueprintResources/StandardMacros.IsValid` _returnvalue
        (:`Is Valid`
          (bind _astestmode (cast `` _returnvalue))
          (`/Engine/EditorBlueprintResources/StandardMacros.IsValid` _astestmode
            (:`Is Valid`
              (bind _asplayer_controller (cast `PlayerController` self))
              (`self.respawn` _astestmode _asplayer_controller))))))))

(fn `UserConstructionScript`)